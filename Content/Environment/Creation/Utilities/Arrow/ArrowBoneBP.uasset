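; Arrow handle at one end of a skeleton in the creation editor that adds or removes bones as it is pushed or pulled.
; Adding extends the skeleton's spline along the drag direction with a slightly smaller bone; removing drops the end bone, both within count limits.
; It then refreshes skin and indices, shifts the spline if within limits, and hands selection to a briefly locked new arrow before destroying itself.
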(fn `AdditionalSelect`
  (params (ActorWhichReplace :type "Actor Object Reference"))
  (bind _utilityskeletonref (`self.UtilitySkeletonRef`))
  (`parent.AdditionalSelect` ActorWhichReplace)
  (if (`self.Selected`)
    (`/Game/Environment/Creation/Utilities/Skeleton/SkeletonBP.Skin Selected` _utilityskeletonref true null)
    (`PrimitiveComponent.SetMaterial` (`self.Arrow`) 0 "/Game/Environment/Materials/Variant/UtilitiesColor/ActorSelected.ActorSelected")
    (else
      (set `/Game/GameplayEntities/Controllers/CreationController.LastSelectedActor` (`/Game/Environment/Creation/Utilities/Skeleton/SkeletonBP.SkinMesh` _utilityskeletonref) (`self.CreationController`)))))

(fn `ArrowIntensityChange`
  (params (Up :type Boolean) (Direction :type "Vector2D Structure"))
  (locals (NewBoneSelected :type "/Game/Environment/Creation/Utilities/Skeleton/BoneBP Object Reference") (IndexNewBone :type Integer))
  (bind (_min _max) (`/Game/GameplayEntities/FunctionsMacros/BoneFunctions.GetStaticMaxMinBoneScale`))
  (bind (_min_2 _max_2) (`/Game/GameplayEntities/FunctionsMacros/BoneFunctions.GetStaticMaxMinBoneScale`))
  (bind _newboneselected (`local.NewBoneSelected`))
  (bind (_direction_x _direction_y) (`KismetMathLibrary.BreakVector2D` (`local.Direction`)))
  (bind (_direction_x_2 _direction_y_2) (`KismetMathLibrary.BreakVector2D` (`local.Direction`)))
  (bind _utilityskeletonref (`self.UtilitySkeletonRef`))
  (bind _uparrow (`self.UpArrow`))
  (bind _skinmesh (`/Game/Environment/Creation/Utilities/Skeleton/SkeletonBP.SkinMesh` (`self.UtilitySkeletonRef`)))
  (bind _bones (`/Game/Environment/Creation/Utilities/Skeleton/SkeletonBP.Bones` (`self.UtilitySkeletonRef`)))
  (bind _arrowref (`/Game/Environment/Creation/Utilities/Skeleton/BoneBP.ArrowRef` (`local.NewBoneSelected`)))
  (bind _skinmesh_2 (`/Game/Environment/Creation/Utilities/Skeleton/SkeletonBP.SkinMesh` (`self.UtilitySkeletonRef`)))
  (bind _spline (`/Game/Environment/Creation/Utilities/Skeleton/SkeletonBP.Spline` (`self.UtilitySkeletonRef`)))
  (bind _returnvalue (`SplineComponent.GetNumberOfSplinePoints` (`/Game/Environment/Creation/Utilities/Skeleton/SkeletonBP.Spline` (`self.UtilitySkeletonRef`))))
  (bind _returnvalue_2 (select `bool` _uparrow :`true` (- _returnvalue 1)))
  (bind _returnvalue_3 (select `bool` (`self.UpArrow`) :`true` (- (`KismetArrayLibrary.Array_Length` _bones) 1)))
  (bind _output (`|GetArrayItem` _bones _returnvalue_3))
  (bind (_returnvalue_x _returnvalue_y _returnvalue_z) (`KismetMathLibrary.BreakVector` (* (`KismetMathLibrary.Normal` (`KismetMathLibrary.MakeVector` _direction_x 0.0 _direction_y)) (* (* (`/Game/GameplayEntities/FunctionsMacros/BoneFunctions.GetStaticBasicBoneDistance`) (`/Game/Environment/Creation/Utilities/Skeleton/BoneBP.Scale` (`|GetArrayItem` (`/Game/Environment/Creation/Utilities/Skeleton/SkeletonBP.Bones` (`self.UtilitySkeletonRef`)) (`/Game/Environment/Creation/Utilities/Skeleton/BoneBP.BoneIndex` (`local.NewBoneSelected`))))) -0.25))))
  (bind _output_2 (`|GetArrayItem` (`/Game/Environment/Creation/Utilities/Skeleton/SkeletonBP.Bones` (`self.UtilitySkeletonRef`)) (+ _returnvalue_2 (select `bool` (`self.UpArrow`) :`false` 1 :`true` -1))))
  (bind _scale (`/Game/Environment/Creation/Utilities/Skeleton/BoneBP.Scale` (`|GetArrayItem` (`/Game/Environment/Creation/Utilities/Skeleton/SkeletonBP.Bones` (`self.UtilitySkeletonRef`)) (select `bool` (`self.UpArrow`) :`true` (- (`SplineComponent.GetNumberOfSplinePoints` (`/Game/Environment/Creation/Utilities/Skeleton/SkeletonBP.Spline` (`self.UtilitySkeletonRef`))) 1)))))
  (if (`self.CanBeUsed`)
    (`parent.ArrowIntensityChange` Up Direction)
    (if (> (`KismetMathLibrary.VSize2D` Direction) 0.3)
      (if (`local.Up`)
        (if (not (`KismetArrayLibrary.Array_IsValidIndex` (`/Game/Environment/Creation/Utilities/Skeleton/SkeletonBP.Bones` (`self.UtilitySkeletonRef`)) (`.Max` (`/Game/GameplayEntities/FunctionsMacros/BoneFunctions.MaxMinBoneNumber`))))
          (`SplineComponent.AddSplinePointAtIndex` (`/Game/Environment/Creation/Utilities/Skeleton/SkeletonBP.Spline` (`self.UtilitySkeletonRef`)) (+ (`self.K2_GetActorLocation` (`self.MasterActor`)) (* (`KismetMathLibrary.Normal` (`KismetMathLibrary.MakeVector` _direction_x_2 0.0 _direction_y_2)) (* (`/Game/GameplayEntities/FunctionsMacros/BoneFunctions.GetStaticBasicBoneDistance`) (`/Game/GameplayEntities/FunctionsMacros/BoneFunctions.GetStaticDistanceWithScaleThanksToBoneScale` _scale (`KismetMathLibrary.FClamp` (- _scale 0.1) _min _max))))) (select `bool` _uparrow :`true` _returnvalue) "World" true)
          (bind _boneref (`/Game/Environment/Creation/Utilities/Skeleton/SkeletonBP.CreateBone` (`self.UtilitySkeletonRef`) _returnvalue_2))
          (set `/Game/Environment/Creation/Utilities/Skeleton/BoneBP.LastRotation` (`/Game/Environment/Creation/Utilities/Skeleton/BoneBP.LastRotation` _output_2) _boneref)
          (set `/Game/Environment/Creation/Utilities/Skeleton/BoneBP.Scale` (`KismetMathLibrary.FClamp` (- (`/Game/Environment/Creation/Utilities/Skeleton/BoneBP.Scale` _output_2) 0.1) _min_2 _max_2) _boneref)
          (`/Engine/EditorBlueprintResources/StandardMacros.IsValid` _skinmesh_2
            (:`Is Valid`
              (`/Game/Environment/Creation/ManipulablePart/Creature/BaseBody/SkinMesh.SpawnSkin` _skinmesh_2 false))
            (:`Is Not Valid`
              _))
          (`/Game/Environment/Creation/Utilities/Skeleton/SkeletonBP.SynchroniseBoneIndex` (`self.UtilitySkeletonRef`) :!label _label)
          (bind _output_get (set `local.NewBoneSelected` _output))
          (`/Game/Environment/Creation/Utilities/Skeleton/BoneBP.SpawnArrowSize` _output_get (`self.UpArrow`))
          (bind _offlimits (`/Game/Environment/Creation/Utilities/Skeleton/SkeletonBP.VerifySplineIsNotOffLimit` (`self.UtilitySkeletonRef`) 0.0 0.0))
          (if _offlimits
            (for (_ _array_index) (`/Game/Environment/Creation/Utilities/Skeleton/SkeletonBP.Bones` _utilityskeletonref)
              (`/Game/Environment/Creation/Utilities/Skeleton/SkeletonBP.MoveSpline` _utilityskeletonref _array_index _returnvalue_x _returnvalue_z)))
          (`/Game/Environment/Creation/Utilities/Skeleton/SkeletonBP.RemoveCollision` (`self.UtilitySkeletonRef`) (`/Game/Environment/Creation/Utilities/Skeleton/BoneBP.BoneIndex` (`local.NewBoneSelected`)))
          (set `/Game/Environment/Creation/Utilities/Arrow/ArrowBP.CanBeUsed` false _arrowref)
          (bind _returnvalue_4 (`KismetSystemLibrary.K2_SetTimer` _arrowref "AllowArrowMove" 0.1))
          (set `/Game/Environment/Creation/Utilities/Arrow/ArrowBP.TimerUsed` _returnvalue_4 _arrowref)
          (`/Game/GameplayEntities/Controllers/CreationController.ChangeAimedActor` (`self.CreationController`) (`/Game/Environment/Creation/Utilities/Skeleton/BoneBP.ArrowRef` (`local.NewBoneSelected`)))
          (`self.SelectActor` _newboneselected false (`/Game/Environment/Creation/Utilities/Skeleton/BoneBP.ArrowRef` _newboneselected))
          (`/Game/GameplayEntities/Controllers/CreationController.Lock Utility` (`self.CreationController`))
          (`self.K2_DestroyActor`))
        (elif (`KismetArrayLibrary.Array_IsValidIndex` (`/Game/Environment/Creation/Utilities/Skeleton/SkeletonBP.Bones` (`self.UtilitySkeletonRef`)) (+ (`/Game/GameplayEntities/FunctionsMacros/BoneFunctions.MaxMinBoneNumber`) 1))
          (`SplineComponent.RemoveSplinePoint` _spline (select `bool` (`self.UpArrow`) :`true` (- (`SplineComponent.GetNumberOfSplinePoints` _spline) 1)) true)
          (`self.K2_DestroyActor` _output)
          (`KismetArrayLibrary.Array_Remove` (`/Game/Environment/Creation/Utilities/Skeleton/SkeletonBP.Bones` (`self.UtilitySkeletonRef`)) _returnvalue_3)
          (`/Engine/EditorBlueprintResources/StandardMacros.IsValid` _skinmesh
            (:`Is Valid`
              (`/Game/Environment/Creation/ManipulablePart/Creature/BaseBody/SkinMesh.SpawnSkin` _skinmesh false)
              (goto _label))
            (:`Is Not Valid`
              (goto _label))))))))

(fn `UserConstructionScript`
  (`parent.UserConstructionScript`))