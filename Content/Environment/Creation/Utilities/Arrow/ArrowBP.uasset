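; Base arrow utility for creation mode, a draggable handle attached to a master actor.
; While locked, Tick projects the camera-relative mouse offset onto the arrow's up vector and, past a threshold, calls the empty ArrowIntensityChange hook with the direction.
; Deselecting destroys the arrow unless the master actor replaces it.
; Unlocking returns the controller's aim to the master actor and toggles its utility lock.
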(event `self.ReceiveTick`
  (params (DeltaSeconds :type "Float (single-precision)"))
  (bind (_xoffset _zoffset) (`/Game/GameplayEntities/FunctionsMacros/MathFunctions.GetMouseOffset` (`self.CreationController`) (`GameplayStatics.GetPlayerCameraManager` 0)))
  (bind (_xoffset_2 _zoffset_2) (`/Game/GameplayEntities/FunctionsMacros/MathFunctions.GetMouseOffset` (`self.CreationController`) (`GameplayStatics.GetPlayerCameraManager` 0)))
  (bind _returnvalue (`KismetMathLibrary.Dot_VectorVector` (`SceneComponent.GetUpVector` (`self.Arrow`)) (`KismetMathLibrary.MakeVector` _xoffset_2 0.0 _zoffset_2)))
  ;[1 1 1] ArrowManipulation
  (if (`self.Locked`)
    (if (> (`KismetMathLibrary.Abs` _returnvalue) 0.3)
      (`self.ArrowIntensityChange` (> _returnvalue 0.0) (`KismetMathLibrary.MakeVector2D` _xoffset _zoffset)))))

(fn `AdditionalLock`
  (bind _creationcontroller (`self.CreationController`))
  (`parent.AdditionalLock`)
  (if (not (`self.Locked`))
    (`/Game/GameplayEntities/Controllers/CreationController.ChangeAimedActor` _creationcontroller (`self.MasterActor`))
    (`/Game/GameplayEntities/Controllers/CreationController.Lock Utility` _creationcontroller)
    (`/Game/GameplayEntities/Controllers/CreationController.UnlockUtility` _creationcontroller)))

(fn `AdditionalSelect`
  (params (ActorWhichReplace :type "Actor Object Reference"))
  (`parent.AdditionalSelect` ActorWhichReplace)
  (if (`self.Selected`)
    _
    (elif (!= ActorWhichReplace (`self.MasterActor`))
      (`self.K2_DestroyActor`))))

(fn `AllowArrowMove`
  (set `self.CanBeUsed` true))

(fn `ArrowIntensityChange`
  (params (Up :type Boolean) (Direction :type "Vector2D Structure")))

(fn `UserConstructionScript`
  ;[1 1 1] MeshRef
  (set `self.MainMesh` (`self.Arrow`)))