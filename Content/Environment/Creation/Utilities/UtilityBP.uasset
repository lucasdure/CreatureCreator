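; UtilityBP is a base actor for creation-mode utilities that can be aimed at, selected and locked.
; It caches the CreationController on BeginPlay and swaps MainMesh's material for aimed and selected states, with aim highlighting suppressed while selected.
; Lock only stores its flag.
; Each aim, select and lock event ends in an empty Additional function, apparently an override hook for child Blueprints.
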(event `/Game/Environment/Creation/Utilities/CreationInterraction.AimActor`
  (params (`Aim/UnAim` :type Boolean))
  (bind _mainmesh (`self.MainMesh`))
  ;[1 1 1] AimActor
  (bind _output_get (set `self.Aimed` `Aim/UnAim`))
  (if (not (`self.Selected`))
    (`/Engine/EditorBlueprintResources/StandardMacros.IsValid` _mainmesh
      (:`Is Valid`
        (`PrimitiveComponent.SetMaterial` _mainmesh 0 (select `bool` _output_get :`false` (`self.UnAimedMat`) :`true` "/Game/Environment/Materials/Variant/UtilitiesColor/ActorAimed.ActorAimed")))
      (:`Is Not Valid`
        _))
    (`self.AdditionialAim`)))

(event `self.ReceiveBeginPlay`
  (`|ExecutionSequence`
    (:`then_0`
      ;[1 1 1] ControllerRef
      (bind _ascreation_controller (cast `/Game/GameplayEntities/Controllers/CreationController` (`GameplayStatics.GetPlayerController` 0)))
      (set `self.CreationController` _ascreation_controller))))

(event `/Game/Environment/Creation/Utilities/CreationInterraction.SelectActor`
  (params (`Select/UnSelect` :type Boolean) (ActorWhichReplace :type "Actor Object Reference"))
  ;[1 1 1] SelectActor
  (bind _output_get (set `self.Selected` `Select/UnSelect`))
  (`PrimitiveComponent.SetMaterial` (`self.MainMesh`) 0 (select `bool` _output_get :`false` (`self.UnAimedMat`) :`true` "/Game/Environment/Materials/Variant/UtilitiesColor/ActorSelected.ActorSelected"))
  (`self.AdditionalSelect` ActorWhichReplace))

(event `/Game/Environment/Creation/Utilities/CreationInterraction.LockActor`
  (params (`Lock/UnLock` :type Boolean))
  ;[1 1 1] LockActor
  (set `self.Locked` `Lock/UnLock`)
  (`self.AdditionalLock`))

(fn `AdditionalLock`)

(fn `AdditionalSelect`
  (params (ActorWhichReplace :type "Actor Object Reference")))

(fn `AdditionialAim`)

(fn `UserConstructionScript`)