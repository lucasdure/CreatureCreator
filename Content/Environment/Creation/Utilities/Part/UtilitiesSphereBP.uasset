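; Sphere utility part in the creation system that passes selection on to its parent actor.
; AdditionalSelect extends the parent logic: when selected it sends a select message to ParentActor, otherwise it records ParentActor as the CreationController's LastSelectedActor.
; AdditionalLock also calls the parent, then deselects the sphere itself if it is not locked.
; The event graph and construction script add no logic of their own.
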(fn `AdditionalLock`
  (`parent.AdditionalLock`)
  (if (not (`self.Locked`))
    (message `/Game/Environment/Creation/Utilities/CreationInterraction.SelectActor` self false null)))

(fn `AdditionalSelect`
  (params (ActorWhichReplace :type "Actor Object Reference"))
  (`parent.AdditionalSelect` ActorWhichReplace)
  (if (`self.Selected`)
    (message `/Game/Environment/Creation/Utilities/CreationInterraction.SelectActor` (`self.ParentActor`) true null)
    (else
      (set `/Game/GameplayEntities/Controllers/CreationController.LastSelectedActor` (`self.ParentActor`) (`self.CreationController`)))))

(fn `UserConstructionScript`
  (`parent.UserConstructionScript`))