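; Draggable sphere handle for the creation tools, letting mouse movement reposition a utility point on its parent actor.
; Each tick while Locked, it offsets its world location by the creation controller's mouse delta along the camera's right and up vectors.
; It sends that proposed location to the parent actor rather than moving itself, and mirrors it with negated world Y to any valid twin utility's parent.
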(event `self.ReceiveTick`
  (params (DeltaSeconds :type "Float (single-precision)"))
  (`parent.ReceiveTick` DeltaSeconds)
  (`self.MoveSphere`))

(fn `MoveSphere`
  (locals (SphereLocation :type "Vector Structure" :default (0.0 0.0 0.0)))
  (bind _returnvalue (`GameplayStatics.GetPlayerCameraManager` 0))
  (bind _twinutility (`self.TwinUtility`))
  (bind (_spherelocation_x _spherelocation_y _spherelocation_z) (`KismetMathLibrary.BreakVector` (`local.SphereLocation`)))
  (bind (_deltax _deltay) (`PlayerController.GetInputMouseDelta` (`self.CreationController`)))
  (if (`self.Locked`)
    (set `local.SphereLocation` (+ (`SceneComponent.K2_GetComponentLocation` (`self.DefaultSceneRoot`)) (* (`self.GetActorRightVector` _returnvalue) _deltax) (* (`self.GetActorUpVector` _returnvalue) _deltay)))
    (message `/Game/Environment/Creation/Utilities/CreationInterraction.SphereUtilityUpdate` (`self.ParentActor`) self (`local.SphereLocation`))
    (`/Engine/EditorBlueprintResources/StandardMacros.IsValid` (`self.TwinUtility`)
      (:`Is Valid`
        (message `/Game/Environment/Creation/Utilities/CreationInterraction.SphereUtilityUpdate` (`/Game/Environment/Creation/Utilities/UtilityBP.ParentActor` _twinutility) _twinutility (`KismetMathLibrary.MakeVector` _spherelocation_x (* _spherelocation_y -1.0) _spherelocation_z))))))

(fn `UserConstructionScript`
  (`parent.UserConstructionScript`))