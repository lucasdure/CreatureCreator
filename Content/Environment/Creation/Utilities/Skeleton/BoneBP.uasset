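; Selectable bone handle for a creation-mode skeleton utility, shown as a sphere that sculpts the owning UtilitySkeleton's spline and skin.
; While locked, it feeds mouse offsets to the skeleton each tick to move its spline point and smooth neighboring bones.
; Zoom input updates the skin scale at its index.
; It extends parent select, lock and aim hooks to swap materials, and can spawn an attached ArrowBoneBP linked back to itself.
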(event `self.ReceiveTick`
  (params (DeltaSeconds :type "Float (single-precision)"))
  (`|ExecutionSequence`
    (:`then_0`
      ;[1 1 1] MoveSplineWhenLocked
      (`self.MoveSplineWIthMouse`))))

(event `self.ZoomInOutUtility`
  (params (Value :type "Float (single-precision)"))
  ;[1 1 1] UpdateSkinScale
  (`/Game/Environment/Creation/Utilities/Skeleton/SkeletonBP.UpdateSkinScaleValue` (`self.UtilitySkeletonRef`) (`self.BoneIndex`) Value)
  (if (!= Value 0.0)
    (`/Game/Environment/Creation/Utilities/Skeleton/SkeletonBP.RemoveCollision` (`self.UtilitySkeletonRef`) (`self.BoneIndex`))
    (`/Game/Environment/Creation/Utilities/Skeleton/SkeletonBP.UpdateSkin` (`self.UtilitySkeletonRef`))))

(fn `AdditionalLock`
  (`parent.AdditionalLock`)
  (if (not (`self.Locked`))
    (set `/Game/GameplayEntities/Controllers/CreationController.LastSelectedActor` null (`self.CreationController`))
    (`self.SelectActor` false self)
    (if (`self.Aimed`)
      (`PrimitiveComponent.SetMaterial` (`self.Sphere`) 0 "/Game/Environment/Materials/Variant/UtilitiesColor/ActorAimed.ActorAimed"))))

(fn `AdditionalSelect`
  (params (ActorWhichReplace :type "Actor Object Reference"))
  (bind _utilityskeletonref (`self.UtilitySkeletonRef`))
  (`parent.AdditionalSelect` ActorWhichReplace)
  (if (`self.Selected`)
    (`/Game/Environment/Creation/Utilities/Skeleton/SkeletonBP.Skin Selected` _utilityskeletonref true null)
    (`PrimitiveComponent.SetMaterial` (`self.Sphere`) 0 "/Game/Environment/Materials/Variant/UtilitiesColor/ActorSelected.ActorSelected")
    (else
      (set `/Game/GameplayEntities/Controllers/CreationController.LastSelectedActor` (`/Game/Environment/Creation/Utilities/Skeleton/SkeletonBP.SkinMesh` _utilityskeletonref) (`self.CreationController`)))))

(fn `AdditionialAim`
  (bind _skinmesh (`/Game/Environment/Creation/Utilities/Skeleton/SkeletonBP.SkinMesh` (`self.UtilitySkeletonRef`)))
  (`parent.AdditionialAim`)
  (`/Engine/EditorBlueprintResources/StandardMacros.IsValid` _skinmesh
    (:`Is Valid`
      (`PrimitiveComponent.SetMaterial` (`self.Sphere`) 0 (select `bool` (`self.Aimed`) :`false` (select `bool` (`/Game/Environment/Creation/Creature/BaseBody/SkinMesh.Selected` _skinmesh) :`false` (`self.UnAimedMat`) :`true` "/Game/Environment/Materials/Variant/Bones/Bones.Bones") :`true` "/Game/Environment/Materials/Variant/UtilitiesColor/ActorAimed.ActorAimed")))))

(fn `GetBoneDistance`
  (returns (Distance :type "Float (double-precision)"))
  (return (* (`self.Scale`) (`/Game/GameplayEntities/FunctionsMacros/BoneFunctions.GetStaticBasicBoneDistance`))))

(fn `MoveSplineWIthMouse`
  (bind (_xoffset _zoffset) (`/Game/GameplayEntities/FunctionsMacros/MathFunctions.GetMouseOffset` (`self.CreationController`) (`GameplayStatics.GetPlayerCameraManager` 0)))
  (if (`self.Locked`)
    (`/Game/Environment/Creation/Utilities/Skeleton/SkeletonBP.MoveSpline` (`self.UtilitySkeletonRef`) (`self.BoneIndex`) _xoffset _zoffset)
    (`/Game/Environment/Creation/Utilities/Skeleton/SkeletonBP.ApplySmoothStrengthToOtherBones` (`self.UtilitySkeletonRef`) (`self.BoneIndex`) (`KismetMathLibrary.MakeVector2D` _xoffset _zoffset))
    (`/Game/Environment/Creation/Utilities/Skeleton/SkeletonBP.RemoveCollision` (`self.UtilitySkeletonRef`) (`self.BoneIndex`))))

(fn `SpawnArrowSize`
  (params (Up :type Boolean))
  (`/Engine/EditorBlueprintResources/StandardMacros.IsValid` (`self.ArrowRef`)
    (:`Is Not Valid`
      (bind _returnvalue (`AddComponent|NODE_AddChildActorComponent-0` :`RelativeTransform` (`KismetMathLibrary.MakeTransform` (select `bool` (`local.Up`) :`false` (-50.0 0.0 0.0) :`true` (50.0 0.0 0.0) :!type "Vector Structure") (select `bool` (`local.Up`) :`false` (struct :`Pitch` 90.0) :`true` (struct :`Pitch` -90.0) :!type "Rotator Structure"))))
      (bind _asarrow_bone_bp (cast `/Game/Environment/Creation/Utilities/Arrow/ArrowBoneBP` (`ChildActorComponent.ChildActor` _returnvalue)))
      (set `self.ArrowRef` _asarrow_bone_bp)
      (set `/Game/Environment/Creation/Utilities/Arrow/ArrowBoneBP.UpArrow` (`local.Up`) _asarrow_bone_bp)
      (set `/Game/Environment/Creation/Utilities/UtilityBP.UtilitySkeletonRef` (`self.UtilitySkeletonRef`) _asarrow_bone_bp)
      (set `/Game/Environment/Creation/Utilities/Arrow/ArrowBP.MasterActor` self _asarrow_bone_bp)
      (`self.K2_AttachToActor` _asarrow_bone_bp self "None" "KeepWorld" "KeepWorld" "KeepWorld" false))))

(fn `UserConstructionScript`
  ;[1 1 1] MeshRef
  (set `self.MainMesh` (`self.Sphere`)))