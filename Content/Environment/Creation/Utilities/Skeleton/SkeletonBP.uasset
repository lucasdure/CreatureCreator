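; Skeleton actor for the creature creation mode that builds a random spine and skin on BeginPlay and registers with CreationController.
; Each spline point drives a BoneBP child actor, and a SkinMesh child follows the bones.
; Spline edits clamp to bounds, propagate with falloff, and enforce bone spacing and angle limits, while dot-product checks correct flipped bones.
; Selecting the skin swaps it to transparent, reveals interactive bones and end arrows, and detaches body parts.
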(event `self.ReceiveBeginPlay`
  (`|ExecutionSequence`
    (:`then_0`
      ;[1 1 1] GenerateRandomBody
      (`self.GenerateRandomBody`))
    (:`then_1`
      ;[1 1 1] GetCreationControllerRef
      (bind _ascreation_controller (cast `/Game/GameplayEntities/Controllers/CreationController` (`GameplayStatics.GetPlayerController` 0)))
      (bind _output_get (set `self.CreationControllerRef` _ascreation_controller))
      (set `/Game/GameplayEntities/Controllers/CreationController.SkeletonRef` self _output_get))))

(fn `AdaptSplinePosition`
  (params (BoneIndex :type Integer))
  (bind (_bonetomodifyup _mainboneup _nextboneup _bonetomodifydown _mainbonedown) (`self.GetUpAndDownBoneIndexInOrder` BoneIndex)
    (:`BoneUpInOrder`
      (`self.BringSplineTogether` _bonetomodifyup _mainboneup))
    (:`BoneDownInOrder`
      (`self.BringSplineTogether` _bonetomodifydown _mainbonedown))))

(fn `ApplySmoothStrengthToOtherBones`
  (params (BoneIndex :type Integer) (InitialStrength :type "Vector2D Structure"))
  (locals (StrengthUpFactor :type Integer :default 0) (StrengthDownFactor :type Integer :default 0) (IndexChoosen :type Integer) (FactorChoosen :type Integer))
  (bind _strengthupfactor (`local.StrengthUpFactor`))
  (bind _strengthdownfactor (`local.StrengthDownFactor`))
  (bind (_returnvalue_x _returnvalue_y) (`KismetMathLibrary.BreakVector2D` (/ (`local.InitialStrength`) (`KismetMathLibrary.MultiplyMultiply_FloatFloat` (`/Game/GameplayEntities/FunctionsMacros/BoneFunctions.GetStaticInfluenceReductionBoneMove`) (`KismetMathLibrary.Conv_IntToDouble` (`local.FactorChoosen`))))))
  (bind (_bonetomodifyup _mainboneup _nextboneup _bonetomodifydown) (`self.GetUpAndDownBoneIndexInOrder` BoneIndex)
    (:`BoneUpInOrder`
      (`/Engine/EditorBlueprintResources/StandardMacros.IncrementInt` _strengthupfactor
        (:`  `
          (set `local.IndexChoosen` _bonetomodifyup)
          (set `local.FactorChoosen` _strengthupfactor))))
    (:`BoneDownInOrder`
      (`/Engine/EditorBlueprintResources/StandardMacros.IncrementInt` _strengthdownfactor
        (:`  `
          (set `local.IndexChoosen` _bonetomodifydown)
          (set `local.FactorChoosen` _strengthdownfactor)))))
  (`self.MoveSpline` (`local.IndexChoosen`) _returnvalue_x _returnvalue_y))

(fn `BringSplineTogether`
  (params (BoneToModify :type Integer) (MainBone :type Integer) (NextBone :type Integer))
  (bind _bones (`self.Bones`))
  (bind _spline (`self.Spline`))
  (bind _returnvalue (`SplineComponent.GetLocationAtSplinePoint` _spline MainBone "World"))
  (`SplineComponent.SetLocationAtSplinePoint` (`self.Spline`) (`local.BoneToModify`) (+ (* (`KismetMathLibrary.Normal` (- (`SplineComponent.GetLocationAtSplinePoint` _spline BoneToModify "World") _returnvalue)) (`/Game/GameplayEntities/FunctionsMacros/BoneFunctions.GetStaticDistanceWithScaleThanksToBoneScale` (`/Game/Environment/Creation/Utilities/Skeleton/BoneBP.GetBoneDistance` (`|GetArrayItem` _bones BoneToModify)) (`/Game/Environment/Creation/Utilities/Skeleton/BoneBP.GetBoneDistance` (`|GetArrayItem` _bones MainBone)))) _returnvalue) "World" true))

(fn `CreateBone`
  (params (BoneIndex :type Integer))
  (returns (BoneRef :type "/Game/Environment/Creation/Utilities/Skeleton/BoneBP Object Reference"))
  (bind _returnvalue (`AddComponent|NODE_AddChildActorComponent-0`))
  (bind _asbone_bp (cast `/Game/Environment/Creation/Utilities/Skeleton/BoneBP` (`ChildActorComponent.ChildActor` _returnvalue)))
  (`KismetArrayLibrary.Array_Insert` (`self.Bones`) _asbone_bp (`local.BoneIndex`))
  (set `/Game/Environment/Creation/Utilities/Skeleton/BoneBP.BoneIndex` (`local.BoneIndex`) _asbone_bp)
  (set `/Game/Environment/Creation/Utilities/Skeleton/BoneBP.Spline` (`self.Spline`) _asbone_bp)
  (set `/Game/Environment/Creation/Utilities/UtilityBP.UtilitySkeletonRef` self _asbone_bp)
  (return _asbone_bp))

(fn `GenerateRandomBody`
  (`self.GenerateRandomBones`)
  (`self.GenerateSkin`))

(fn `GenerateRandomBones`
  (locals (RandomIntToUse :type Integer :default 0))
  (bind (_min _max) (`/Game/GameplayEntities/FunctionsMacros/BoneFunctions.MaxMinBoneNumber`))
  (bind _bones (`self.Bones`))
  (`|ExecutionSequence`
    (:`then_0`
      (`KismetArrayLibrary.Array_Clear` (`self.Bones`))
      (`SplineComponent.ClearSplinePoints` (`self.Spline`) true)
      (bind _output_get (set `local.RandomIntToUse` (`KismetMathLibrary.RandomIntegerInRange` _min _max)))
      (for _index (range (+ _output_get 1))
        (`SplineComponent.AddPoint` (`self.Spline`) (make `SplinePoint` (`KismetMathLibrary.Conv_IntToDouble` _index) (* (`KismetMathLibrary.MakeVector` 0.0 0.0 (`/Game/GameplayEntities/FunctionsMacros/BoneFunctions.GetStaticBasicBoneDistance`)) _index)) false)
        (bind _boneref (`self.CreateBone` _index))
        (set `/Game/Environment/Creation/Utilities/Skeleton/BoneBP.Scale` (`KismetMathLibrary.RandomFloatInRange` (`/Game/GameplayEntities/FunctionsMacros/BoneFunctions.GetStaticMaxMinBoneScale`) 1.2) _boneref))
      (`SplineComponent.UpdateSpline` (`self.Spline`)))
    (:`then_1`
      (`self.UpdateBonesPosition` false)
      (for (_ _array_index) (`self.Bones`)
        (`self.RotateBone180` _array_index)
        (`self.UpdateBoneLastRotation` _array_index)))
    (:`then_2`
      (`/Game/Environment/Creation/Utilities/Skeleton/BoneBP.SpawnArrowSize` (`|GetArrayItem` _bones) false)
      (`/Game/Environment/Creation/Utilities/Skeleton/BoneBP.SpawnArrowSize` (`|GetArrayItem` _bones (- (`KismetArrayLibrary.Array_Length` (`self.Bones`)) 1)) true))
    (:`then_3`
      (for (_ _array_index_2) (`self.Bones`)
        (`self.MoveSpline` _array_index_2 (`KismetMathLibrary.RandomFloatInRange` -10.0 10.0))
        (`self.RemoveCollision` _array_index_2)))))

(fn `GenerateSkin`
  (locals (IndexLocal :type Integer))
  (`self.GenerateSkinMaterials`)
  (bind _returnvalue (`AddComponent|NODE_AddChildActorComponent-4`))
  (bind _asskin_mesh (cast `/Game/Environment/Creation/ManipulablePart/Creature/BaseBody/SkinMesh` (`ChildActorComponent.ChildActor` _returnvalue)))
  (bind _output_get (set `self.SkinMesh` _asskin_mesh))
  (set `/Game/Environment/Creation/ManipulablePart/Creature/BaseBody/SkinMesh.SkeletonRef` self _output_get)
  (`/Game/Environment/Creation/ManipulablePart/Creature/BaseBody/SkinMesh.SpawnSkin` _output_get false))

(fn `GenerateSkinMaterials`
  (bind _returnvalue (`KismetMaterialLibrary.CreateDynamicMaterialInstance` "/Game/Environment/Materials/Variant/Parts/Creature/CreatureSkinOpaque.CreatureSkinOpaque"))
  (set `self.SkinOpaque` _returnvalue)
  (bind _returnvalue_2 (`KismetMaterialLibrary.CreateDynamicMaterialInstance` "/Game/Environment/Materials/Variant/Parts/Creature/CreatureSkinTransparent.CreatureSkinTransparent"))
  (set `self.SkinTransparent` _returnvalue_2))

(fn `GetSmoothAngle`
  (params (BoneIndex :type Integer))
  (locals (LocalIndex :type Integer) (MainBone :type Integer))
  (set `local.MainBone` BoneIndex)
  (for _index (range 1 (+ (- (`SplineComponent.GetNumberOfSplinePoints` (`self.Spline`)) 2) 1))
    (bind _output_get (set `local.LocalIndex` _index))
    (if (!= _output_get (`local.MainBone`))
      (`self.ResetInCaseOfHardAngle` _output_get))))

(fn `Is Bone Rotation Wrong`
  (params (IndexToVerify :type Integer) (CompareWithOther :type Boolean) (OnlyNext :type Boolean) (LastIndex :type Integer))
  (returns (Wrong :type Boolean))
  (bind _indextoverify (`local.IndexToVerify`))
  (bind _output (`|GetArrayItem` (`self.Bones`) IndexToVerify))
  (bind _returnvalue (`self.GetActorUpVector` _output))
  (bind _returnvalue_2 (< (`KismetMathLibrary.Dot_VectorVector` _returnvalue (`self.GetActorUpVector` (`|GetArrayItem` (`self.Bones`) (+ IndexToVerify -1)))) 0.0))
  (bind _returnvalue_3 (< (`KismetMathLibrary.Dot_VectorVector` (`self.GetActorUpVector` (`|GetArrayItem` (`self.Bones`) (+ IndexToVerify 1))) _returnvalue) 0.0))
  (if (not (`local.CompareWithOther`))
    (return (< (`KismetMathLibrary.Dot_VectorVector` (`self.GetActorUpVector` _output) (`KismetMathLibrary.GetUpVector` (`/Game/Environment/Creation/Utilities/Skeleton/BoneBP.LastRotation` _output))) 0.0))
    (elif (== _indextoverify (`local.LastIndex`))
      (return (and _returnvalue_2 (not (`local.OnlyNext`))))
      (elif (or (== _indextoverify 0) (`local.OnlyNext`))
        (return _returnvalue_3)
        (else
          (return (and _returnvalue_3 _returnvalue_2)))))))

(fn `MoveAllBonesInDirection`
  (bind (_xoffset _zoffset) (`/Game/GameplayEntities/FunctionsMacros/MathFunctions.GetMouseOffset` (`self.CreationControllerRef`) (`GameplayStatics.GetPlayerCameraManager` 0)))
  (bind _returnvalue (/ _zoffset 2.0))
  (bind _returnvalue_2 (/ _xoffset 2.0))
  (bind _offlimits (`self.VerifySplineIsNotOffLimit` _returnvalue_2 _returnvalue))
  (if (not _offlimits)
    (for (_ _array_index) (`self.Bones`)
      (`self.MoveSpline` _array_index _returnvalue_2 _returnvalue))
    (`self.UpdateBonesPosition` false)))

(fn `MoveSpline`
  (params (BoneIndex :type Integer) (XOffset :type "Float (double-precision)") (ZOffset :type "Float (double-precision)"))
  (bind (_xmin _xmax _zmin _zmax) (`/Game/GameplayEntities/FunctionsMacros/BoneFunctions.GetStaticMaxMinBonePosition`))
  (bind (_returnvalue_x _returnvalue_y _returnvalue_z) (`KismetMathLibrary.BreakVector` (`SplineComponent.GetLocationAtSplinePoint` (`self.Spline`) BoneIndex "World")))
  (bind _returnvalue (/ (`/Game/GameplayEntities/FunctionsMacros/BoneFunctions.GetStaticBasicBoneDistance`) 5.0))
  (`SplineComponent.SetLocationAtSplinePoint` (`self.Spline`) (`local.BoneIndex`) (`KismetMathLibrary.MakeVector` (`KismetMathLibrary.FClamp` (+ _returnvalue_x (* (`local.XOffset`) _returnvalue)) _xmin _xmax) 0.0 (`KismetMathLibrary.FClamp` (+ _returnvalue_z (* (`local.ZOffset`) _returnvalue)) _zmin _zmax)) "World" true))

(fn `RemoveCollision`
  (params (BoneIndex :type Integer))
  (`self.ResetInCaseOfHardAngle` BoneIndex true)
  (`self.GetSmoothAngle` BoneIndex)
  (`self.AdaptSplinePosition` BoneIndex)
  (`self.Verify Spline Are Not To Closes` BoneIndex)
  (`self.UpdateBonesPosition` false))

(fn `ResetInCaseOfHardAngle`
  (params (BoneIndex :type Integer) (ReverseDirection :type Boolean))
  (locals (MainIndex :type Integer) (Offset :type "Vector Structure" :default (0.0 0.0 0.0)))
  (bind _distancetoreturn (`/Game/GameplayEntities/FunctionsMacros/BoneFunctions.GetStaticMaxAngle`))
  (bind _spline (`self.Spline`))
  (bind _returnvalue (`SplineComponent.GetLocationAtSplinePoint` _spline (`local.MainIndex`) "World"))
  (bind _returnvalue_2 (- (`KismetMathLibrary.FindClosestPointOnSegment` _returnvalue (`SplineComponent.GetLocationAtSplinePoint` _spline (- (`local.MainIndex`) 1) "World") (`SplineComponent.GetLocationAtSplinePoint` _spline (+ (`local.MainIndex`) 1) "World")) _returnvalue))
  (bind _returnvalue_3 (`KismetMathLibrary.VSize` _returnvalue_2))
  (set `local.MainIndex` BoneIndex)
  (if (> _returnvalue_3 _distancetoreturn)
    (set `local.Offset` (* (`KismetMathLibrary.Normal` _returnvalue_2) (- _returnvalue_3 _distancetoreturn)))
    (if (`local.ReverseDirection`)
      (for _index (range (`SplineComponent.GetNumberOfSplinePoints` (`self.Spline`)))
        (if (!= _index (`local.MainIndex`))
          (`SplineComponent.SetLocationAtSplinePoint` (`self.Spline`) _index (- (`SplineComponent.GetLocationAtSplinePoint` (`self.Spline`) _index "World") (`local.Offset`)) "World" false)))
      (else
        (`SplineComponent.SetLocationAtSplinePoint` (`self.Spline`) (`local.MainIndex`) (+ _returnvalue (`local.Offset`)) "World" false)))))

(fn `RotateBone180`
  (params (BoneIndex :type Integer))
  (bind _output (`|GetArrayItem` (`self.Bones`) BoneIndex))
  (`self.K2_SetActorRotation` _output (`KismetMathLibrary.ComposeRotators` (`self.K2_GetActorRotation` _output) (`KismetMathLibrary.RotatorFromAxisAndAngle` (`self.GetActorForwardVector` _output) 180.0)) false))

(fn `SetBonesInterractable`
  (params (Visible :type Boolean))
  (bind _returnvalue (select `bool` Visible :`false` "ECR_Ignore" :`true` "ECR_Block" :!type "ECollisionResponse Enum"))
  (bind _bones (`self.Bones`))
  (for _array_element (`self.Bones`)
    (bind _sphere (`/Game/Environment/Creation/Utilities/Skeleton/BoneBP.Sphere` _array_element))
    (`PrimitiveComponent.SetCollisionResponseToChannel` _sphere "ECC_GameTraceChannel2" _returnvalue)
    (`PrimitiveComponent.SetCollisionResponseToChannel` _sphere "ECC_GameTraceChannel1" _returnvalue))
  (`PrimitiveComponent.SetCollisionResponseToChannel` (`/Game/Environment/Creation/Utilities/Arrow/ArrowBP.Arrow` (`/Game/Environment/Creation/Utilities/Skeleton/BoneBP.ArrowRef` (`|GetArrayItem` _bones))) "ECC_GameTraceChannel1" _returnvalue)
  (`PrimitiveComponent.SetCollisionResponseToChannel` (`/Game/Environment/Creation/Utilities/Arrow/ArrowBP.Arrow` (`/Game/Environment/Creation/Utilities/Skeleton/BoneBP.ArrowRef` (`|GetArrayItem` _bones (- (`KismetArrayLibrary.Array_Length` _bones) 1)))) "ECC_GameTraceChannel1" _returnvalue))

(fn `SetBonesVisible`
  (params (Visible :type Boolean))
  (bind _bones (`self.Bones`))
  (bind _arrowref (`/Game/Environment/Creation/Utilities/Skeleton/BoneBP.ArrowRef` (`|GetArrayItem` _bones)))
  (bind _returnvalue (select `bool` Visible :`false` "/Game/Environment/Materials/Effect/Invisible.Invisible" :`true` (`/Game/Environment/Creation/Utilities/UtilityBP.UnAimedMat` _arrowref)))
  (for _array_element (`self.Bones`)
    (`PrimitiveComponent.SetMaterial` (`/Game/Environment/Creation/Utilities/Skeleton/BoneBP.Sphere` _array_element) 0 (select `bool` Visible :`false` "/Game/Environment/Materials/Effect/Invisible.Invisible" :`true` (`/Game/Environment/Creation/Utilities/UtilityBP.UnAimedMat` _array_element))))
  (`PrimitiveComponent.SetMaterial` (`/Game/Environment/Creation/Utilities/Arrow/ArrowBP.Arrow` _arrowref) 0 _returnvalue)
  (`PrimitiveComponent.SetMaterial` (`/Game/Environment/Creation/Utilities/Arrow/ArrowBP.Arrow` (`/Game/Environment/Creation/Utilities/Skeleton/BoneBP.ArrowRef` (`|GetArrayItem` _bones (- (`KismetArrayLibrary.Array_Length` _bones) 1)))) 0 _returnvalue))

(fn `Skin Selected`
  (params (Select :type Boolean) (ActorWhichReplace :type "Actor Object Reference"))
  (bind _skinmesh (`self.SkinMesh`))
  (`self.SetBonesVisible` Select)
  (`self.SetBonesInterractable` Select)
  (`/Engine/EditorBlueprintResources/StandardMacros.IsValid` _skinmesh
    (:`Is Valid`
      (if (not (== Select (`/Game/Environment/Creation/ManipulablePart/Creature/BaseBody/SkinMesh.Selected` _skinmesh)))
        (bind _output_get (set `/Game/Environment/Creation/ManipulablePart/Creature/BaseBody/SkinMesh.Selected` Select _skinmesh))
        (`PrimitiveComponent.SetMaterial` (`Character.Mesh` (`self.SkinMesh`)) 0 (select `bool` _output_get :`false` (`self.SkinOpaque`) :`true` (`self.SkinTransparent`) :!type "MaterialInterface Object Reference"))
        (`/Game/Environment/Creation/ManipulablePart/Creature/BaseBody/SkinMesh.StartAnimation` (`self.SkinMesh`) (not (`local.Select`)))
        (`PrimitiveComponent.SetCustomDepthStencilValue` (`Character.Mesh` (`self.SkinMesh`)) (select `bool` (`local.Select`)))
        (for _array_element (`/Game/Environment/Creation/ManipulablePart/Creature/BaseBody/SkinMesh.BodyParts` (`self.SkinMesh`))
          (`/Game/Environment/Creation/ManipulablePart/ManipulablePartBP.SetAttached` _array_element (not (`local.Select`)))
          (bind _twin (`/Game/Environment/Creation/ManipulablePart/ManipulablePartBP.Twin` _array_element))
          (`/Engine/EditorBlueprintResources/StandardMacros.IsValid` _twin
            (:`Is Valid`
              (`/Game/Environment/Creation/ManipulablePart/ManipulablePartBP.SetAttached` _twin (not (`local.Select`))))))))))

(fn `SkinAimed`
  (params (Aimed :type Boolean) (ActorWhichReplace :type "Actor Object Reference"))
  (bind _skinmesh (`self.SkinMesh`))
  (`/Engine/EditorBlueprintResources/StandardMacros.IsValid` _skinmesh
    (:`Is Valid`
      (if (not (== Aimed (`/Game/Environment/Creation/ManipulablePart/Creature/BaseBody/SkinMesh.Aimed` _skinmesh)))
        (bind _output_get (set `/Game/Environment/Creation/ManipulablePart/Creature/BaseBody/SkinMesh.Aimed` Aimed _skinmesh))
        (`PrimitiveComponent.SetCustomDepthStencilValue` (`Character.Mesh` (`self.SkinMesh`)) (select `bool` _output_get :`true` 1))))))

(fn `SkinLocked`
  (params (Locked :type Boolean))
  (set `/Game/Environment/Creation/ManipulablePart/Creature/BaseBody/SkinMesh.Locked` Locked (`self.SkinMesh`)))

(fn `SynchroniseBoneIndex`
  (for (_array_element _array_index) (`self.Bones`)
    (set `/Game/Environment/Creation/Utilities/Skeleton/BoneBP.BoneIndex` _array_index _array_element)))

(fn `UpdateBoneLastRotation`
  (params (BoneIndex :type Integer))
  (bind _output (`|GetArrayItem` (`self.Bones`) BoneIndex))
  (set `/Game/Environment/Creation/Utilities/Skeleton/BoneBP.LastRotation` (`self.K2_GetActorRotation` _output) _output))

(fn `UpdateBonesPosition`
  (params (IgnoreSkin :type Boolean))
  (locals (LastIndex :type Integer :default 0) (LocalIndex :type Integer))
  (bind _spline (`self.Spline`))
  (bind _bones (`self.Bones`))
  (bind _localindex (`local.LocalIndex`))
  (bind _localindex_2 (`local.LocalIndex`))
  (bind _localindex_3 (`local.LocalIndex`))
  (`|ExecutionSequence`
    (:`then_0`
      (set `local.LastIndex` (- (`KismetArrayLibrary.Array_Length` _bones) 1))
      (for (_array_element _array_index) _bones
        (set `local.LocalIndex` _array_index)
        (`self.K2_SetActorTransform` _array_element (`KismetMathLibrary.MakeTransform` (`SplineComponent.GetLocationAtSplinePoint` _spline (`local.LocalIndex`) "World") (`KismetMathLibrary.MakeRotFromX` (- (`SplineComponent.GetLocationAtSplinePoint` _spline (+ (`local.LocalIndex`) (select `bool` (== (`local.LocalIndex`) (`local.LastIndex`)) :`false` 1)) "World") (`SplineComponent.GetLocationAtSplinePoint` _spline (- (`local.LocalIndex`) (select `bool` (== (`local.LocalIndex`) 0) :`false` 1)) "World")))) false false)
        (if (`self.Is Bone Rotation Wrong` (`local.LocalIndex`) false false (`local.LastIndex`))
          (`self.RotateBone180` _localindex))
        (`self.UpdateBoneLastRotation` _localindex)))
    (:`then_1`
      (for (_ _array_index_2) (`self.Bones`)
        (bind _output_get (set `local.LocalIndex` _array_index_2))
        (if (`self.Is Bone Rotation Wrong` _output_get true false (`local.LastIndex`))
          (`self.RotateBone180` _localindex_3))
        (`self.UpdateBoneLastRotation` _localindex_3)))
    (:`then_2`
      (for (_ _array_index_3) (`self.Bones`)
        (bind _output_get_2 (set `local.LocalIndex` _array_index_3))
        (if (`self.Is Bone Rotation Wrong` _output_get_2 true true (`local.LastIndex`))
          (`self.RotateBone180` _localindex_2))
        (`self.UpdateBoneLastRotation` _localindex_2)))
    (:`then_3`
      (if (not (`local.IgnoreSkin`))
        (`self.UpdateSkin`)))))

(fn `UpdateSkin`
  (locals (LocalIndex :type Integer) (Change :type Boolean))
  (bind _skinmesh (`self.SkinMesh`))
  (`/Engine/EditorBlueprintResources/StandardMacros.IsValid` _skinmesh
    (:`Is Valid`
      (`/Game/Environment/Creation/ManipulablePart/Creature/BaseBody/SkinMesh.UpdateSkin` _skinmesh))))

(fn `UpdateSkinScaleValue`
  (params (LocalIndex :type Integer) (Value :type "Float (double-precision)"))
  (bind (_min _max) (`/Game/GameplayEntities/FunctionsMacros/BoneFunctions.GetStaticMaxMinBoneScale`))
  (bind _output (`|GetArrayItem` (`self.Bones`) LocalIndex))
  (if (`KismetArrayLibrary.Array_IsValidIndex` (`self.Bones`) LocalIndex)
    (set `/Game/Environment/Creation/Utilities/Skeleton/BoneBP.Scale` (`KismetMathLibrary.FClamp` (+ (`/Game/Environment/Creation/Utilities/Skeleton/BoneBP.Scale` _output) (/ Value 10.0)) _min _max) _output)))

(fn `UserConstructionScript`)

(fn `Verify Spline Are Not To Closes`
  (params (BoneIndex :type Integer))
  (locals (IndexLocal :type Integer) (MainBone :type Integer))
  (bind _spline (`self.Spline`))
  (bind _bones (`self.Bones`))
  (bind _returnvalue (`SplineComponent.GetLocationAtSplinePoint` _spline (`local.MainBone`) "World"))
  (bind _returnvalue_2 (- (`SplineComponent.GetLocationAtSplinePoint` _spline (`local.IndexLocal`) "World") _returnvalue))
  (bind _distance (`/Game/GameplayEntities/FunctionsMacros/BoneFunctions.GetStaticDistanceWithScaleThanksToBoneScale` (`/Game/Environment/Creation/Utilities/Skeleton/BoneBP.GetBoneDistance` (`|GetArrayItem` _bones (`local.IndexLocal`))) (`/Game/Environment/Creation/Utilities/Skeleton/BoneBP.GetBoneDistance` (`|GetArrayItem` _bones (`local.MainBone`)))))
  (for _index (range (`SplineComponent.GetNumberOfSplinePoints` (`self.Spline`)))
    (set `local.MainBone` _index)
    (for _index_2 (range (`SplineComponent.GetNumberOfSplinePoints` (`self.Spline`)))
      (if (not (== (`local.MainBone`) _index_2))
        (set `local.IndexLocal` _index_2)
        (if (< (`KismetMathLibrary.VSize` _returnvalue_2) (- _distance 0.01))
          (`SplineComponent.SetLocationAtSplinePoint` (`self.Spline`) (`local.IndexLocal`) (+ (* (`KismetMathLibrary.Normal` _returnvalue_2) _distance) _returnvalue) "World" true))))))

(fn `VerifySplineIsNotOffLimit`
  (params (XOffset :type "Float (double-precision)") (ZOffset :type "Float (double-precision)"))
  (returns (OffLimits :type Boolean))
  (bind (_xmin _xmax _zmin _zmax) (`/Game/GameplayEntities/FunctionsMacros/BoneFunctions.GetStaticMaxMinBonePosition`))
  (bind _returnvalue (/ (`/Game/GameplayEntities/FunctionsMacros/BoneFunctions.GetStaticBasicBoneDistance`) 5.0))
  (for _index (range (`SplineComponent.GetNumberOfSplinePoints` (`self.Spline`)))
    (bind (_returnvalue_x _returnvalue_y _returnvalue_z) (`KismetMathLibrary.BreakVector` (`SplineComponent.GetLocationAtSplinePoint` (`self.Spline`) _index "World")))
    (bind _returnvalue_2 (+ _returnvalue_x (* (`local.XOffset`) _returnvalue)))
    (bind _returnvalue_3 (+ _returnvalue_z (* (`local.ZOffset`) _returnvalue)))
    (if (not (and (>= _returnvalue_2 _xmin) (<= _returnvalue_2 _xmax) (>= _returnvalue_3 _zmin) (<= _returnvalue_3 _zmax)))
      (return true)))
  (return false))