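; BodyBaseBP is the base body actor for creatures, handling aim, select and lock interactions.
; Its AimActor, SelectActor and LockActor events forward their state to the Skeleton component, which handles the skin's response, including the replacing actor passed on selection.
; While Locked is true, Tick calls MoveAllBonesInDirection on the Skeleton to move the whole body base.
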(event `self.ReceiveTick`
  (params (DeltaSeconds :type "Float (single-precision)"))
  ;[1 1 1] MoveBodyBaseOnly
  (if (`self.Locked`)
    (`/Game/Environment/Creation/Utilities/Skeleton/SkeletonBP.MoveAllBonesInDirection` (`self.Skeleton`))))

(event `/Game/Environment/Creation/Utilities/CreationInteraction.AimActor`
  (params (`Aim/UnAim` :type Boolean))
  ;[1 1 1] SkinAimed
  (`/Game/Environment/Creation/Utilities/Skeleton/SkeletonBP.SkinAimed` (`self.Skeleton`) `Aim/UnAim` null))

(event `/Game/Environment/Creation/Utilities/CreationInteraction.SelectActor`
  (params (`Select/UnSelect` :type Boolean) (ActorWhichReplace :type "Actor Object Reference"))
  ;[1 1 1] SelectSkin
  (`/Game/Environment/Creation/Utilities/Skeleton/SkeletonBP.Skin Selected` (`self.Skeleton`) `Select/UnSelect` ActorWhichReplace))

(event `/Game/Environment/Creation/Utilities/CreationInteraction.LockActor`
  (params (`Lock/UnLock` :type Boolean))
  ;[1 1 1] LockSkin
  (`/Game/Environment/Creation/Utilities/Skeleton/SkeletonBP.SkinLocked` (`self.Skeleton`) `Lock/UnLock`))

(fn `UserConstructionScript`)