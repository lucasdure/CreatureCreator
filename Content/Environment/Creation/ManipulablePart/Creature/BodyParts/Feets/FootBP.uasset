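; FootBP is a manipulable foot body part for creature creation, attached to a creature's legs.
; Each tick it snaps to the "Foot" socket on the legs' SimpleSkeleton, adding a stored transform offset.
; Aiming sets the mesh's custom depth stencil as a highlight, and zoom input resizes the foot within fixed bounds.
; Both highlight and scale changes are mirrored to its Twin foot when one exists.
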(event `self.ReceiveTick`
  (params (DeltaSeconds :type "Float (single-precision)"))
  (`self.CorrectLocRot`))

(event `/Game/Environment/Creation/Utilities/CreationInterraction.ZoomInOutUtility`
  (params (Value :type "Float (single-precision)"))
  ;[1 1 1] UpdateSkinScale
  (`self.UpdateFootScale` Value))

(fn `Aim`
  (params (Aim :type Boolean))
  (bind _twin (`self.Twin`))
  (`parent.Aim` Aim)
  (`PrimitiveComponent.SetCustomDepthStencilValue` (`self.Foot`) (select `bool` (`self.Aimed`) :`true` 1))
  (`/Engine/EditorBlueprintResources/StandardMacros.IsValid` _twin
    (:`Is Valid`
      (bind _asfoot_bp (cast `/Game/Environment/Creation/ManipulablePart/Creature/BodyParts/Feets/FootBP` _twin))
      (`PrimitiveComponent.SetCustomDepthStencilValue` (`/Game/Environment/Creation/ManipulablePart/Creature/BodyParts/Feets/FootBP.Foot` _asfoot_bp) (select `bool` (`self.Aimed`) :`true` 1)))))

(fn `CorrectLocRot`
  (bind _legsref (`self.LegsRef`))
  (bind (_transformoffset_location _transformoffset_rotation) (`KismetMathLibrary.BreakTransform` (`self.TransformOffset`)))
  (bind (_returnvalue_location _returnvalue_rotation) (`KismetMathLibrary.BreakTransform` (`SceneComponent.GetSocketTransform` (`/Game/Environment/Creation/ManipulablePart/Creature/BodyParts/Eyes/SimpleSkeletonMesh.SimpleSkeleton` _legsref) "Foot" "RTS_World")))
  (`/Engine/EditorBlueprintResources/StandardMacros.IsValid` _legsref
    (:`Is Valid`
      (`self.K2_SetActorLocationAndRotation` (+ _transformoffset_location _returnvalue_location) (`KismetMathLibrary.ComposeRotators` _transformoffset_rotation _returnvalue_rotation)))))

(fn `UpdateFootScale`
  (params (Value :type "Float (double-precision)"))
  (locals (NewScale :type "Vector Structure" :default (0.0 0.0 0.0)))
  (bind _twin (`self.Twin`))
  (bind _returnvalue (+ (`KismetMathLibrary.Conv_DoubleToVector` (* Value 0.04)) (`SceneComponent.K2_GetComponentScale` (`self.Foot`))))
  (bind _x (.x _returnvalue))
  (if (and (< _x 1.5) (> _x 0.5))
    (bind _output_get (set `local.NewScale` _returnvalue))
    (`self.SetActorScale3D` _output_get)
    (`/Engine/EditorBlueprintResources/StandardMacros.IsValid` _twin
      (:`Is Valid`
        (`self.SetActorScale3D` _twin (`local.NewScale`))))))

(fn `UserConstructionScript`)