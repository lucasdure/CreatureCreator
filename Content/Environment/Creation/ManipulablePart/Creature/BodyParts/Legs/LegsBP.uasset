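; Leg body part for the creature creator that stretches or bends to reach the ground and carries a foot child actor.
; Each tick it zeroes leg rotation and traces down to drive LegAnimation's section positions.
; When attached or skin is moving, ground distance bends the knee against the stored length; otherwise it sets that length.
; Overrides of parent functions pass skin material, skeleton and twin links to the feet and manage custom-stencil highlighting.
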(event `self.ReceiveBeginPlay`
  (`parent.ReceiveBeginPlay`)
  (`|ExecutionSequence`
    (:`then_0`
      ;[1 1 1] AnimationRef
      (bind _asleg_animation (cast `/Game/Environment/Creation/ManipulablePart/Creature/BodyParts/Legs/LegAnimation` (`SkeletalMeshComponent.GetAnimInstance` (`self.Leg`))))
      (set `self.AnimRef` _asleg_animation))
    (:`then_1`
      ;[1 1 1] GetKneeRatio
      (`self.Get Knee Ratio`))))

(event `self.ReceiveTick`
  (params (DeltaSeconds :type "Float (single-precision)"))
  ;[1 1 1] ResetRotation
  (`self.ResetRotation`)
  ;[1 1 1] DetectLegLength
  (`self.GetLegsLength`))

(fn `Aim`
  (params (Aim :type Boolean))
  (bind _twin (`self.Twin`))
  (`parent.Aim` Aim)
  (`PrimitiveComponent.SetCustomDepthStencilValue` (`self.Leg`) (select `bool` (`self.Aimed`) :`true` 1))
  (`/Engine/EditorBlueprintResources/StandardMacros.IsValid` _twin
    (:`Is Valid`
      (bind _aslegs_bp (cast `/Game/Environment/Creation/ManipulablePart/Creature/BodyParts/Legs/LegsBP` _twin))
      (`PrimitiveComponent.SetCustomDepthStencilValue` (`/Game/Environment/Creation/ManipulablePart/Creature/BodyParts/Legs/LegsBP.Leg` _aslegs_bp) (select `bool` (`self.Aimed`) :`true` 1)))))

(fn `AttachFeet`
  (params (FootClass :type "/Game/Environment/Creation/ManipulablePart/Creature/BodyParts/Feets/FootBP Class Reference"))
  (`ChildActorComponent.SetChildActorClass` (`self.Foot`) FootClass)
  (bind _asfoot_bp (cast `/Game/Environment/Creation/ManipulablePart/Creature/BodyParts/Feets/FootBP` (`ChildActorComponent.ChildActor` (`self.Foot`))))
  (bind _output_get (set `self.FootRef` _asfoot_bp))
  (set `/Game/Environment/Creation/ManipulablePart/Creature/BodyParts/Feets/FootBP.LegsRef` self _output_get)
  (`/Game/Environment/Creation/ManipulablePart/Creature/BodyParts/Feets/FootBP.CorrectLocRot` _output_get))

(fn `AttachToSkeletonWithTwin `
  (params (SkeletonRef :type "/Game/Environment/Creation/Utilities/Skeleton/SkeletonBP Object Reference"))
  (bind _twin (`self.Twin`))
  (`parent.AttachToSkeletonWithTwin ` SkeletonRef)
  (set `/Game/Environment/Creation/ManipulablePart/ManipulablePartBP.SkinMeshRef` (`self.SkinMeshRef`) (`self.FootRef`))
  (`/Engine/EditorBlueprintResources/StandardMacros.IsValid` _twin
    (:`Is Valid`
      (bind _aslegs_bp (cast `/Game/Environment/Creation/ManipulablePart/Creature/BodyParts/Legs/LegsBP` _twin))
      (set `/Game/Environment/Creation/ManipulablePart/ManipulablePartBP.SkinMeshRef` (`self.SkinMeshRef`) (`/Game/Environment/Creation/ManipulablePart/Creature/BodyParts/Legs/LegsBP.FootRef` _aslegs_bp)))))

(fn `ChangeSkinMaterial`
  (params (MaterialInterface :type "MaterialInterface Object Reference"))
  (`parent.ChangeSkinMaterial` MaterialInterface)
  (`PrimitiveComponent.SetMaterial` (`self.Leg`) 0 (`local.MaterialInterface`))
  (`PrimitiveComponent.SetMaterial` (`/Game/Environment/Creation/ManipulablePart/Creature/BodyParts/Feets/FootBP.Foot` (`self.FootRef`)) 0 (`local.MaterialInterface`)))

(fn `Get Knee Ratio`
  (bind _returnvalue_location (`KismetMathLibrary.BreakTransform` (`SceneComponent.GetSocketTransform` (`self.Leg`) "UpLeg" "RTS_World")))
  (bind _returnvalue_location_2 (`KismetMathLibrary.BreakTransform` (`SceneComponent.GetSocketTransform` (`self.Leg`) "UpLeg" "RTS_World")))
  (bind (_returnvalue_x _returnvalue_y _returnvalue_z) (`KismetMathLibrary.BreakVector` (- _returnvalue_location (`SceneComponent.K2_GetComponentLocation` (`self.Knee`)))))
  (bind (_returnvalue_x_2 _returnvalue_y_2 _returnvalue_z_2) (`KismetMathLibrary.BreakVector` (- (`SceneComponent.K2_GetComponentLocation` (`Actor.RootComponent` (`self.FootRef`))) _returnvalue_location_2)))
  (set `self.KneeRatio` (`KismetMathLibrary.Abs` (/ _returnvalue_z _returnvalue_z_2))))

(fn `GetLegsLength`
  (bind (_middlesectionposition_x _middlesectionposition_y) (`KismetMathLibrary.BreakVector` (`self.MiddleSectionPosition`)))
  (bind (_lastsectionposition_x _lastsectionposition_y) (`KismetMathLibrary.BreakVector` (`self.LastSectionPosition`)))
  (bind _animref (`self.AnimRef`))
  (bind (_middlesectionposition_x_2 _middlesectionposition_y_2) (`KismetMathLibrary.BreakVector` (`self.MiddleSectionPosition`)))
  (bind (_lastsectionposition_x_2 _lastsectionposition_y_2) (`KismetMathLibrary.BreakVector` (`self.LastSectionPosition`)))
  (bind _animref_2 (`self.AnimRef`))
  (bind _returnvalue (`SceneComponent.K2_GetComponentLocation` (`self.Leg`)))
  (bind _footlength (`/Game/Environment/Creation/ManipulablePart/Creature/CreatureAnimation.FootLength` _animref))
  (bind _outhit (`KismetSystemLibrary.LineTraceSingleForObjects` _returnvalue (+ _returnvalue (0.0 0.0 -10000.0)) (`|MakeArray` "ObjectTypeQuery1" :!type "EObjectTypeQuery Enum") true))
  (bind (_bblockinghit _binitialoverlap _time _distance) (`GameplayStatics.BreakHitResult` _outhit))
  (if _bblockinghit
    (set `self.LegLength` (`KismetMathLibrary.FMax` _distance 1.0))
    (if (`self.AttachedOrMovingSkin`)
      (set `/Game/Environment/Creation/ManipulablePart/Creature/CreatureAnimation.Foot Distance` (`self.LegLength`) (`self.AnimRef`))
      (set `/Game/Environment/Creation/ManipulablePart/Creature/CreatureAnimation.MiddleSectionPosition` (`KismetMathLibrary.MakeVector` (* (/ (+ (* (- (`/Game/Environment/Creation/ManipulablePart/Creature/CreatureAnimation.Foot Distance` _animref) _footlength) (/ _footlength -100.0)) (`/Game/Environment/Creation/ManipulablePart/Creature/CreatureAnimation.FootLength` (`self.AnimRef`))) (`self.OffsetTopOfGround`)) _middlesectionposition_x) _middlesectionposition_y (* -1.0 (- (`/Game/Environment/Creation/ManipulablePart/Creature/CreatureAnimation.Foot Distance` _animref_2) (* (`/Game/Environment/Creation/ManipulablePart/Creature/CreatureAnimation.FootLength` _animref_2) 0.55)))) (`self.AnimRef`))
      (set `/Game/Environment/Creation/ManipulablePart/Creature/CreatureAnimation.LastSectionPosition` (`KismetMathLibrary.MakeVector` _lastsectionposition_x _lastsectionposition_y (* -1.0 (`/Game/Environment/Creation/ManipulablePart/Creature/CreatureAnimation.Foot Distance` (`self.AnimRef`)))) (`self.AnimRef`))
      (else
        (set `/Game/Environment/Creation/ManipulablePart/Creature/CreatureAnimation.FootLength` (`self.LegLength`) (`self.AnimRef`))
        (set `/Game/Environment/Creation/ManipulablePart/Creature/CreatureAnimation.MiddleSectionPosition` (`KismetMathLibrary.MakeVector` (* (/ (`/Game/Environment/Creation/ManipulablePart/Creature/CreatureAnimation.FootLength` (`self.AnimRef`)) (`self.OffsetTopOfGround`)) _middlesectionposition_x_2) _middlesectionposition_y_2 (* -0.45 (`/Game/Environment/Creation/ManipulablePart/Creature/CreatureAnimation.FootLength` (`self.AnimRef`)))) (`self.AnimRef`))
        (set `/Game/Environment/Creation/ManipulablePart/Creature/CreatureAnimation.LastSectionPosition` (`KismetMathLibrary.MakeVector` _lastsectionposition_x_2 _lastsectionposition_y_2 (* -1.0 (`/Game/Environment/Creation/ManipulablePart/Creature/CreatureAnimation.FootLength` (`self.AnimRef`)))) (`self.AnimRef`))))))

(fn `Lock`
  (params (Lock :type Boolean))
  (bind _twin (`self.Twin`))
  (`parent.Lock` Lock)
  (`PrimitiveComponent.SetCustomDepthStencilValue` (`self.Leg`) 0)
  (`/Engine/EditorBlueprintResources/StandardMacros.IsValid` _twin
    (:`Is Valid`
      (bind _aslegs_bp (cast `/Game/Environment/Creation/ManipulablePart/Creature/BodyParts/Legs/LegsBP` _twin))
      (`PrimitiveComponent.SetCustomDepthStencilValue` (`/Game/Environment/Creation/ManipulablePart/Creature/BodyParts/Legs/LegsBP.Leg` _aslegs_bp) 0))))

(fn `ResetRotation`
  (`SceneComponent.K2_SetWorldRotation` :`self` (`self.Leg`)))

(fn `Update Twin Ref`
  (params (FuturTwinRef :type "/Game/Environment/Creation/ManipulablePart/ManipulablePartBP Object Reference"))
  (`parent.Update Twin Ref` FuturTwinRef)
  (bind _aslegs_bp (cast `/Game/Environment/Creation/ManipulablePart/Creature/BodyParts/Legs/LegsBP` (`self.Twin`)))
  (bind _footref (`/Game/Environment/Creation/ManipulablePart/Creature/BodyParts/Legs/LegsBP.FootRef` _aslegs_bp))
  (bind _output_get (set `/Game/Environment/Creation/ManipulablePart/ManipulablePartBP.Twin` (`self.FootRef`) _footref))
  (bind _output_get_2 (set `/Game/Environment/Creation/ManipulablePart/ManipulablePartBP.Twin` _footref _output_get))
  (`self.SetActorScale3D` _output_get_2 (`self.GetActorScale3D` (`self.FootRef`))))

(fn `UserConstructionScript`
  (`self.AttachFeet` "/Game/Environment/Creation/ManipulablePart/Creature/BodyParts/Feets/SimpleFoot/SimpleFootBp.SimpleFootBp_C"))