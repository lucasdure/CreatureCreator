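; BodyPartBP is a creature body part in the creation system's manipulable part hierarchy.
; It extends the parent's attach and clear logic to keep the skin mesh's BodyParts list in sync.
; Attaching to a skeleton without a twin adds the part to that skeleton's SkinMesh list.
; Clearing only this part removes it from SkinMeshRef's list, if valid, before the parent logic runs.
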(fn `AttachToSkeletonWithoutTwin`
  (params (SkeletonRef :type "/Game/Environment/Creation/Utilities/Skeleton/SkeletonBP Object Reference"))
  (`parent.AttachToSkeletonWithoutTwin` SkeletonRef)
  (`KismetArrayLibrary.Array_Add` (`/Game/Environment/Creation/ManipulablePart/Creature/BaseBody/SkinMesh.BodyParts` (`/Game/Environment/Creation/Utilities/Skeleton/SkeletonBP.SkinMesh` (`local.SkeletonRef`))) self))

(fn `ClearOnlyManipulablePart`
  (bind _skinmeshref (`self.SkinMeshRef`))
  (`/Engine/EditorBlueprintResources/StandardMacros.IsValid` _skinmeshref
    (:`Is Valid`
      (`KismetArrayLibrary.Array_RemoveItem` (`/Game/Environment/Creation/ManipulablePart/Creature/BaseBody/SkinMesh.BodyParts` _skinmeshref) self))
    (:`Is Not Valid`
      _))
  (`parent.ClearOnlyManipulablePart`))

(fn `UserConstructionScript`)