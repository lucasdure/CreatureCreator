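; EyesBP is the Blueprint for an eyes body part of a creature, built around a SimpleSkeleton mesh component.
; On BeginPlay it casts the skeleton's anim instance to EyeAnimBP and stores it in AnimRef.
; ChangeSkinMaterial swaps the given material into the skeleton's second material slot.
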(event `self.ReceiveBeginPlay`
  (`parent.ReceiveBeginPlay`)
  (`|ExecutionSequence`
    (:`then_0`
      ;[1 1 1] AnimationRef
      (bind _aseye_anim_bp (cast `/Game/Environment/Creation/ManipulablePart/Creature/BodyParts/Eyes/EyeAnimBP` (`SkeletalMeshComponent.GetAnimInstance` (`self.SimpleSkeleton`))))
      (set `self.AnimRef` _aseye_anim_bp))))

(fn `ChangeSkinMaterial`
  (params (MaterialInterface :type "MaterialInterface Object Reference"))
  (`PrimitiveComponent.SetMaterial` (`self.SimpleSkeleton`) 1 (`local.MaterialInterface`)))

(fn `UserConstructionScript`
  (`parent.UserConstructionScript`))