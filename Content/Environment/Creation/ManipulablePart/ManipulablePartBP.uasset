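; Base actor for parts the player manipulates in the creature creation mode, tracking aimed, selected, locked and attached states.
; A part attaches to the closest skin mesh bone, and a linked twin mirrors attachment, selection and aimed attach points.
; Locking, or mouse movement while locked, detaches the part and hands it to the CreationController.
; Attach points toggle collision and widgets by part type, with empty functions left as hooks.
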(event `self.ReceiveBeginPlay`
  ;[1 1 1] ControllerRef
  (bind _ascreation_controller (cast `/Game/GameplayEntities/Controllers/CreationController` (`GameplayStatics.GetPlayerController` 0)))
  (set `self.CreationController` _ascreation_controller))

(event `/Game/Environment/Creation/Utilities/CreationInterraction.AimActor`
  (params (`Aim/UnAim` :type Boolean))
  ;[1 1 1] PartAimed
  (`self.Aim` `Aim/UnAim`))

(event `/Game/Environment/Creation/Utilities/CreationInterraction.SelectActor`
  (params (`Select/UnSelect` :type Boolean) (ActorWhichReplace :type "Actor Object Reference"))
  ;[1 1 1] PartSelected
  (`self.Select Manipulable Part` `Select/UnSelect` ActorWhichReplace))

(event `self.ReceiveTick`
  (params (DeltaSeconds :type "Float (single-precision)"))
  (bind (_deltax _deltay) (`PlayerController.GetInputMouseDelta` (`self.CreationController`)))
  ;[1 1 1] Detach if mouse move
  (if (and (`self.Locked`) (`self.LockOnlyWhenMouseMove`) (not (`self.AttachedOrMovingSkin`)))
    (if (> (+ (`KismetMathLibrary.Abs` _deltax) (`KismetMathLibrary.Abs` _deltay)) 0.3)
      (`self.DetachFromBody`))))

(event `/Game/Environment/Creation/Utilities/CreationInterraction.LockActor`
  (params (`Lock/UnLock` :type Boolean))
  ;[1 1 1] PartLocked
  (`self.Lock` `Lock/UnLock`))

(fn `Aim`
  (params (Aim :type Boolean))
  (set `self.Aimed` Aim))

(fn `AttachedPointAimed`
  (params (AttachAimed :type Boolean) (AttachPointTag :type Name) (IsTwin :type Boolean))
  (bind _twin (`self.Twin`))
  (if (not IsTwin)
    (`/Engine/EditorBlueprintResources/StandardMacros.IsValid` _twin
      (:`Is Valid`
        (`self.AttachedPointAimed` _twin AttachAimed AttachPointTag true)))))

(fn `AttachToSkeletonWithoutTwin`
  (params (SkeletonRef :type "/Game/Environment/Creation/Utilities/Skeleton/SkeletonBP Object Reference"))
  (bind _output_get (set `self.BoneAtttached` (`.ReturnValue` (`SkinnedMeshComponent.FindClosestBone_K2` (`Character.Mesh` (`/Game/Environment/Creation/Utilities/Skeleton/SkeletonBP.SkinMesh` (`local.SkeletonRef`))) (`self.K2_GetActorLocation`) 0.0 false))))
  (`self.K2_AttachToComponent` (`Character.Mesh` (`/Game/Environment/Creation/Utilities/Skeleton/SkeletonBP.SkinMesh` (`local.SkeletonRef`))) _output_get "KeepWorld" "KeepWorld" "KeepWorld")
  (set `self.SkinMeshRef` (`/Game/Environment/Creation/Utilities/Skeleton/SkeletonBP.SkinMesh` (`local.SkeletonRef`)))
  (`self.SetAttached` true)
  (set `self.Locked` false))

(fn `AttachToSkeletonWithTwin `
  (params (SkeletonRef :type "/Game/Environment/Creation/Utilities/Skeleton/SkeletonBP Object Reference") (FuturParentActor :type "Actor Object Reference"))
  (bind _twin (`self.Twin`))
  (`self.AttachToSkeletonWithoutTwin` self (`local.SkeletonRef`))
  (`/Engine/EditorBlueprintResources/StandardMacros.IsValid` _twin
    (:`Is Valid`
      (`self.AttachToSkeletonWithoutTwin` _twin (`local.SkeletonRef`)))))

(fn `ChangeSkinMaterial`
  (params (MaterialInterface :type "MaterialInterface Object Reference")))

(fn `ClearManipulablePartAndTwin`
  (bind _twin (`self.Twin`))
  (`/Engine/EditorBlueprintResources/StandardMacros.IsValid` _twin
    (:`Is Valid`
      (`self.ClearOnlyManipulablePart` _twin))
    (:`Is Not Valid`
      _))
  (`self.ClearOnlyManipulablePart`))

(fn `ClearOnlyManipulablePart`
  (`self.K2_DestroyActor`))

(fn `DetachFromBody`
  (bind _twin (`self.Twin`))
  (`self.NotifyMeshParentIfAttached`)
  (`self.Select Manipulable Part` false)
  (`/Game/GameplayEntities/Controllers/CreationController.Create Part` (`self.CreationController`) (`GameplayStatics.GetObjectClass` self))
  (set `PlayerController.bShowMouseCursor` true (`self.CreationController`))
  (set `/Game/GameplayEntities/Controllers/CreationController.SpawnedPart` self (`self.CreationController`))
  (set `/Game/GameplayEntities/Controllers/CreationController.LastAimedActor` null (`self.CreationController`))
  (`self.SetAttached` self false)
  (bind _asbody_part_bp (cast `/Game/Environment/Creation/ManipulablePart/Creature/BodyParts/BodyPartBP` self)
    (:`then`
      (`KismetArrayLibrary.Array_RemoveItem` (`/Game/Environment/Creation/ManipulablePart/Creature/BaseBody/SkinMesh.BodyParts` (`self.SkinMeshRef`)) _asbody_part_bp))
    (:`CastFailed`
      _))
  (`/Engine/EditorBlueprintResources/StandardMacros.IsValid` _twin
    (:`Is Valid`
      (`self.SetAttached` _twin false)
      (bind _asbody_part_bp_2 (cast `/Game/Environment/Creation/ManipulablePart/Creature/BodyParts/BodyPartBP` (`self.Twin`))
        (:`then`
          (`KismetArrayLibrary.Array_RemoveItem` (`/Game/Environment/Creation/ManipulablePart/Creature/BaseBody/SkinMesh.BodyParts` (`self.SkinMeshRef`)) _asbody_part_bp_2))
        (:`CastFailed`
          _)))
    (:`Is Not Valid`
      _))
  (`/Game/Environment/Creation/ManipulablePart/Creature/BaseBody/SkinMesh.RevealAllAttachs` (`self.SkinMeshRef`) (`self.PartType`) true false))

(fn `Lock`
  (params (Lock :type Boolean))
  (bind _output_get (set `self.Locked` Lock))
  (if (and _output_get (not (`self.LockOnlyWhenMouseMove`)))
    (`self.DetachFromBody`)))

(fn `NotifyMeshParentIfAttached`)

(fn `RevealAttachPoint`
  (params (PartTypeToReveal :type "/Game/Environment/Creation/ManipulablePart/Creature/PartType Enum" :default "NewEnumerator0") (Reveal :type Boolean) (VisualOnly :type Boolean))
  (locals (Index :type Integer) (Valid :type Boolean :default false))
  (bind _output (`|GetArrayItem` (`self.AttachPartList`) (`local.Index`)))
  (bind ((`WidgetComponentRef_8_519CDAA74686BD927CC983A3AD2FB8F3` _widgetcomponentref)) (break `/Game/Environment/Creation/Utilities/Structure/AttachInParts` (`|GetArrayItem` (`self.AttachPartList`) (`local.Index`))))
  (for (_ _array_index) (`self.AttachPartList`)
    (set `local.Index` _array_index)
    (set `local.Valid` (and (`|EnumEquality` (`.PartType_2_A35253304E8ECE9C89438390C6708C8B` (break `/Game/Environment/Creation/Utilities/Structure/AttachInParts` (`|GetArrayItem` (`self.AttachPartList`) (`local.Index`)))) (`local.PartTypeToReveal`)) (`local.Reveal`)))
    (if (not (`local.VisualOnly`))
      (`PrimitiveComponent.SetCollisionEnabled` (`.PrimitiveComponentRef_5_EDF45D57455E52E17B196CB0093698BD` (break `/Game/Environment/Creation/Utilities/Structure/AttachInParts` (`|GetArrayItem` (`self.AttachPartList`) (`local.Index`)))) (select `bool` (`local.Valid`) :`false` "NoCollision" :`true` "QueryOnly" :!type "ECollisionEnabled Enum")))
    (if (`local.Valid`)
      (`/Engine/EditorBlueprintResources/StandardMacros.IsValid` (`.WidgetComponentRef_8_519CDAA74686BD927CC983A3AD2FB8F3` (break `/Game/Environment/Creation/Utilities/Structure/AttachInParts` (`|GetArrayItem` (`self.AttachPartList`) (`local.Index`))))
        (:`Is Not Valid`
          (bind _returnvalue (`AddComponent|NODE_AddWidgetComponent-0`))
          (setmembers `/Game/Environment/Creation/Utilities/Structure/AttachInParts` :`StructRef` _output :`WidgetComponentRef` _returnvalue)
          (`SceneComponent.K2_SetWorldLocation` _returnvalue (`SceneComponent.K2_GetComponentLocation` (`.PrimitiveComponentRef_5_EDF45D57455E52E17B196CB0093698BD` (break `/Game/Environment/Creation/Utilities/Structure/AttachInParts` _output))) false false)))
      (else
        (`/Engine/EditorBlueprintResources/StandardMacros.IsValid` _widgetcomponentref
          (:`Is Valid`
            (`ActorComponent.K2_DestroyComponent` _widgetcomponentref))
          (:`Is Not Valid`
            _))
        (setmembers `/Game/Environment/Creation/Utilities/Structure/AttachInParts` :`StructRef` (`|GetArrayItem` (`self.AttachPartList`) (`local.Index`)) :`WidgetComponentRef` null)))))

(fn `Select`
  (params (Selected :type Boolean) (ActorWhichReplace :type "Actor Object Reference"))
  (set `self.Selected` Selected))

(fn `Select Manipulable Part`
  (params (Select :type Boolean) (ActorWhichReplace :type "Actor Object Reference"))
  (bind _twin (`self.Twin`))
  (bind _skinmeshref (`self.SkinMeshRef`))
  (`/Engine/EditorBlueprintResources/StandardMacros.IsValid` _skinmeshref
    (:`Is Valid`
      (`/Game/Environment/Creation/Utilities/Skeleton/SkeletonBP.StartCreatureAnimation` (`/Game/Environment/Creation/ManipulablePart/Creature/BaseBody/SkinMesh.SkeletonRef` _skinmeshref) (not Select)))
    (:`Is Not Valid`
      _))
  (`self.Select` Select (`local.ActorWhichReplace`))
  (`/Engine/EditorBlueprintResources/StandardMacros.IsValid` _twin
    (:`Is Valid`
      (`self.Select` _twin Select (`local.ActorWhichReplace`)))))

(fn `SetAttached`
  (params (AttachedOrMovingSkin :type Boolean))
  (set `self.AttachedOrMovingSkin` AttachedOrMovingSkin))

(fn `Update Twin Ref`
  (params (FuturTwinRef :type "/Game/Environment/Creation/ManipulablePart/ManipulablePartBP Object Reference"))
  (bind _output_get (set `self.Twin` FuturTwinRef))
  (set `/Game/Environment/Creation/ManipulablePart/ManipulablePartBP.Twin` self _output_get)
  (set `/Game/Environment/Creation/ManipulablePart/ManipulablePartBP.SecondPart` true _output_get))

(fn `UserConstructionScript`)